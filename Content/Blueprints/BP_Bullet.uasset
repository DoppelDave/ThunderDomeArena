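; BP_Bullet is a bullet actor that flies straight along its forward vector.
; BeginPlay teleports it 175 units upward, then Tick advances it by BulletSpeed scaled by delta time.
; Movement uses SetActorLocation without sweep, and the file holds no hit or overlap handling.
; A MoveActor function offers the same movement for any speed and direction, but the event graph does not call it.
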(event `self.ReceiveBeginPlay`
  (`self.K2_SetActorLocation` (+ (`self.K2_GetActorLocation`) (0.0 0.0 175.0)) false true))

(event `self.ReceiveTick`
  (params (DeltaSeconds :type "Float (single-precision)"))
  (`self.K2_SetActorLocation` (+ (* (* (`self.bulletSpeed`) DeltaSeconds) (`KismetMathLibrary.Conv_RotatorToVector` (`self.K2_GetActorRotation`))) (`self.K2_GetActorLocation`))))

(fn `MoveActor`
  (params (speed :type "Float (single-precision)") (direction :type "Vector Structure") (deltatime :type "Float (double-precision)"))
  (`self.K2_SetActorLocation` (+ (`self.K2_GetActorLocation`) (* (* direction deltatime) speed))))

(fn `UserConstructionScript`)