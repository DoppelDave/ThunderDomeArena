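; Drivable car actor that moves, turns and shoots from driving, turn and fire state variables set outside this file.
; Tick accelerates or applies friction using Data tuning values, adds a clamped yaw step, and moves the car forward without sweep or physics.
; It spawns BP_Bullet every frame while shooting and toggles weapon visibility.
; Car tiers swap by hiding meshes; BeginPlay hides level 2, and UpgradeCar's call is unwired.
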(event `self.ReceiveBeginPlay`
  (`self.InitializeCar`))

(event `self.ReceiveTick`
  (params (DeltaSeconds :type "Float (single-precision)"))
  (bind _currentrotation (`self.currentRotation`))
  (bind (_data_maxspeed _data_acceleration _data_brakeforce _data_friction _data_rotationspeed) (break `/Game/Blueprints/CarData` (`self.data`)))
  (if (`self.isDriving`)
    (`self.Accelerate Object` DeltaSeconds _data_maxspeed _data_acceleration)
    (else
      (`self.Friction Object` DeltaSeconds _data_friction)))
  (set `self.currentRotation` (`KismetMathLibrary.FClamp` (+ (* (* _data_rotationspeed DeltaSeconds) (`self.turnInput`)) _currentrotation) -1.0))
  (`self.K2_SetActorRotation` (`KismetMathLibrary.ComposeRotators` (`self.K2_GetActorRotation`) (`KismetMathLibrary.MakeRotator` 0.0 0.0 _currentrotation)))
  (`self.K2_SetActorLocation` (+ (`self.K2_GetActorLocation`) (* (* (`self.currentSpeed`) DeltaSeconds) (`KismetMathLibrary.GreaterGreater_VectorRotator` (`KismetMathLibrary.Vector_Forward`) (`self.K2_GetActorRotation`)))))
  (if (`self.isShooting`)
    (`|SpawnActorFromClass` "/Game/Blueprints/BP_Bullet.BP_Bullet_C" (`self.GetTransform`) "AlwaysSpawn" "MultiplyWithRoot" null null))
  (if (`self.hasNextWeapon`)
    (`SceneComponent.SetHiddenInGame` (`self.BP_Weapon_1`) true false)
    (`SceneComponent.SetHiddenInGame` (`self.BP_Weapon_2`) false false)
    (else
      (`SceneComponent.SetHiddenInGame` (`self.BP_Weapon_2`) true false))))

(fn `Accelerate Object`
  (params (DeltaSeconds :type "Float (double-precision)") (MaxSpeed :type "Float (double-precision)") (Acceleration :type "Float (double-precision)"))
  (bind _currentspeed (`self.currentSpeed`))
  (set `self.currentSpeed` (+ (`self.currentSpeed`) (* Acceleration DeltaSeconds)))
  (set `self.currentSpeed` (`KismetMathLibrary.FClamp` _currentspeed _currentspeed MaxSpeed)))

(fn `DowngradeCar`
  (`SceneComponent.SetHiddenInGame` (`self.car_2_Base_2`) true false)
  (`SceneComponent.SetHiddenInGame` (`self.car_2_Top_2`) true false)
  (`SceneComponent.SetHiddenInGame` (`self.Car_1_Top_1`) false false)
  (`SceneComponent.SetHiddenInGame` (`self.Car_1_Base_1`) false false))

(fn `Friction Object`
  (params (Deltatime :type "Float (double-precision)") (Friction :type "Float (double-precision)"))
  (bind _frictionforce (`self.frictionForce`))
  (bind _currentspeed (`self.currentSpeed`))
  (set `self.frictionForce` (* Friction Deltatime))
  (if (> _currentspeed 0.0)
    (set `self.currentSpeed` (`KismetMathLibrary.FClamp` _currentspeed 0.0 (- _currentspeed _frictionforce)))
    (else
      (set `self.currentSpeed` (`KismetMathLibrary.FClamp` _currentspeed 0.0 (+ _frictionforce _currentspeed))))))

(fn `InitializeCar`
  ;[1 1 1] Hide CarLevel2 Gear
  (`SceneComponent.SetHiddenInGame` (`self.car_2_Top_2`) true false)
  (`SceneComponent.SetHiddenInGame` (`self.car_2_Base_2`) true false))

(fn `UpgradeCar`
  (`SceneComponent.SetHiddenInGame` (`self.Car_1_Top_1`) true false)
  (`SceneComponent.SetHiddenInGame` (`self.Car_1_Base_1`) true false)
  (`SceneComponent.SetHiddenInGame` (`self.car_2_Top_2`) false false)
  (`SceneComponent.SetHiddenInGame` (`self.car_2_Base_2`) false false))

(fn `UserConstructionScript`)