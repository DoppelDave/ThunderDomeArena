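; InputController forwards player driving, turning and shooting input to the InputActor pawn.
; On BeginPlay it casts player 0's pawn to InputActor and caches the reference.
; Accelerate and Shoot presses and releases toggle the actor's IsDriving and IsShooting flags.
; The Turn axis feeds TurnInput and resets CurrentRotation when it returns to zero, so this Blueprint only writes state to the actor.
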(event `self.ReceiveBeginPlay`
  (bind _asinput_actor (cast `/Game/Blueprints/Input/InputActor` (`GameplayStatics.GetPlayerPawn` 0)))
  (set `self.inputActor` _asinput_actor))

(event `InputAction|Accelerate`
  (params (Key :type "Key Structure"))
  (:`Pressed`
    (bind _inputactor (`self.inputActor`)
      (:`then`
        (set `/Game/Blueprints/Input/InputActor.isDriving` true _inputactor))
      (:`else`)))
  (:`Released`
    (bind _inputactor_2 (`self.inputActor`)
      (:`then`
        (set `/Game/Blueprints/Input/InputActor.isDriving` false _inputactor_2))
      (:`else`))))

(event `InputAxis|Turn`
  (params (AxisValue :type "Float (single-precision)"))
  (bind _inputactor (`self.inputActor`)
    (:`then`
      (set `/Game/Blueprints/Input/InputActor.turnInput` AxisValue _inputactor)
      (if (== AxisValue 0.0)
        (set `/Game/Blueprints/Input/InputActor.currentRotation` 0.0 _inputactor)))
    (:`else`)))

(event `InputAction|Shoot`
  (params (Key :type "Key Structure"))
  (:`Pressed`
    (bind _inputactor (`self.inputActor`)
      (:`then`
        (set `/Game/Blueprints/Input/InputActor.isShooting` true _inputactor))
      (:`else`)))
  (:`Released`
    (bind _inputactor_2 (`self.inputActor`)
      (:`then`
        (set `/Game/Blueprints/Input/InputActor.isShooting` false _inputactor_2))
      (:`else`))))

(fn `UserConstructionScript`)